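; Openable door actor that swings open and shut in response to the OpenDoor component's open and close events.
; A DoorSwing timeline drives a yaw offset combined with the rotation saved at BeginPlay.
; Opening plays a sound and is gated by a DoOnce, which closing resets while reversing the timeline.
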(event OnClose(OpenDoor)
  (Utilities|FlowControl|Sequence
    (:then_0
      (bind _door_open_angle (Timeline|Door%20Swing Reverse)
        (:Update
          (Transformation|SetActorRotation (Math|Rotator|CombineRotators (Math|Rotator|MakeRotator 0.0 0.0 _door_open_angle) (Variables|Default|GetInitial%20Rotation))))))
    (:then_1
      (Utilities|FlowControl|DoOnce false) ; enters at Reset
    )))

(event OnOpen(OpenDoor)
  (Utilities|FlowControl|DoOnce false
    (:Completed
      (Audio|PlaySoundatLocation (Variables|Default|GetDoor%20Open%20Sound) (Transformation|GetActorLocation) "0, 0, 0" 1.0 1.0 0.0 0 0 0)
      (bind _door_open_angle (Timeline|Door%20Swing Play)
        (:Update
          (Transformation|SetActorRotation (Math|Rotator|CombineRotators (Math|Rotator|MakeRotator 0.0 0.0 _door_open_angle) (Variables|Default|GetInitial%20Rotation))))))))

(event EventBeginPlay
  (Variables|Default|SetInitial%20Rotation (Transformation|GetActorRotation)))

(fn ConstructionScript)